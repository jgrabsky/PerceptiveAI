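; Guard NPC character that carries a weapon, exposes AI state hooks and ragdolls on death.
; On BeginPlay it spawns its weapon class and attaches it to the mesh's weapon socket.
; State events forward changes to the animation instance and set walk speed per AI state, while getters expose death status, patrol route and team ID.
; The health component's death event switches the mesh to physics ragdoll and disables capsule collision, guarded by DoOnce.
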(event `self.ReceiveBeginPlay`
  (bind _returnvalue (`|SpawnActorFromClass` (`self.WeaponClass`) (`/Game/Blueprints/Shared/Library_BP.IdentityTransform`) "AlwaysSpawn" "OverrideRootScale" self self))
  (bind _output_get (set `self.Weapon` _returnvalue))
  (`self.K2_AttachToComponent` (`self.Weapon`) (`self.Mesh`) "WeaponSocket" "SnapToTarget" "SnapToTarget" "SnapToTarget" true)
  (`self.K2_AttachToComponent` _output_get (`self.Mesh`) "WeaponSocket" "SnapToTarget" "SnapToTarget" "SnapToTarget" true))

(event `self.Health_BP.OnDamageTaken`)

(event `self.Health_BP.OnDeath`
  (bind _mesh (`self.Mesh`))
  ;[1 1 1] On Death
  (`/Engine/EditorBlueprintResources/StandardMacros.DoOnce` false
    (:`Completed`
      (`PrimitiveComponent.SetCollisionProfileName` _mesh "Ragdoll" true)
      (`SkeletalMeshComponent.SetAllBodiesSimulatePhysics` _mesh true)
      (`PrimitiveComponent.WakeAllRigidBodies` _mesh)
      (`PrimitiveComponent.SetCollisionEnabled` (`self.CapsuleComponent`) "NoCollision")
      (`KismetSystemLibrary.PrintString` (`KismetStringLibrary.Concat_StrStr` (`KismetSystemLibrary.GetDisplayName` self) " Died!")))))

(event `/Game/Blueprints/Shared/AI_BPI.NotifyStateChanged`
  (params (NewState :type "/Game/AI/NPC_State_E Enum" :default "NewEnumerator0"))
  ;[1 1 1] On State Changed
  (message `/Game/Blueprints/Shared/AI_BPI.NotifyStateChanged` (`SkeletalMeshComponent.GetAnimInstance` (`self.Mesh`)) NewState))

(event `/Game/Blueprints/Shared/AI_BPI.ModifyMovementSpeed`
  (params (State :type "/Game/AI/NPC_State_E Enum" :default "NewEnumerator0"))
  (set `CharacterMovementComponent.MaxWalkSpeed` (select `/Game/AI/NPC_State_E` State :`NewEnumerator0` 160.0 :`NewEnumerator1` 160.0 :`NewEnumerator2` 400.0 :`NewEnumerator3` 600.0 :`NewEnumerator4` 0.0 :!type "Float (single-precision)") (`self.CharacterMovement`)))

(fn `GetIsDead`
  (returns (Dead :type Boolean))
  (return (`/Game/Blueprints/Shared/Health_BP.IsDead` (`self.Health_BP`))))

(fn `GetPatrolRoute`
  (returns (PatrolRoute :type "/Game/Blueprints/NPC/PatrolRoute Object Reference"))
  (return (`self.MyPatrolPath`)))

(fn `GetTeamID`
  (returns (IsPlayer :type Boolean))
  (return false))

(fn `UserConstructionScript`)