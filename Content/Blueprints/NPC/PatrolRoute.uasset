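; PatrolRoute is a Blueprint that defines a looping patrol path, apparently for NPCs, using a PatrolPath spline.
; It tracks a PatrolIndex, and GetNextPointAsWorldPosition returns the world location of the spline point at that index.
; IncrementPatrolPath advances the index and wraps it to the first point with a modulo on the point count.
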(event `IncrementPatrolPath`
  (set `self.PatrolIndex` (mod (+ (`self.PatrolIndex`) 1) (`SplineComponent.GetNumberOfSplinePoints` (`self.PatrolPath`)))))

(fn `GetNextPointAsWorldPosition`
  (returns (ReturnValue :type "Vector Structure"))
  (return (`SplineComponent.GetLocationAtSplinePoint` (`self.PatrolPath`) (`self.PatrolIndex`) "World")))

(fn `UserConstructionScript`)